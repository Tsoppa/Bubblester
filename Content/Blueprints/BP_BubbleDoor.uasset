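; BP_BubbleDoor is an exit door actor that ends the game once nothing remains to be completed.
; On BeginPlay it caches the third-person game mode.
; When the player character overlaps its box and the game mode's Remaining count is zero, it pauses the game, shows the mouse cursor and displays the WB_EndingMenu widget.
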(event `self.ReceiveBeginPlay`
  (bind _asbp_third_person_game_mode (cast `/Game/ThirdPerson/Blueprints/BP_ThirdPersonGameMode` (`GameplayStatics.GetGameMode`)))
  (set `self.As BP Third Person Game Mode` _asbp_third_person_game_mode))

(event `self.Box.OnComponentBeginOverlap`
  (params (OverlappedComponent :type "PrimitiveComponent Object Reference") (OtherActor :type "Actor Object Reference") (OtherComp :type "PrimitiveComponent Object Reference") (OtherBodyIndex :type Integer) (bFromSweep :type Boolean) (SweepResult :type "HitResult Structure (by ref)"))
  (if (== OtherActor (`GameplayStatics.GetPlayerCharacter` 0))
    (if (== (`/Game/ThirdPerson/Blueprints/BP_ThirdPersonGameMode.Remaining` (`self.As BP Third Person Game Mode`)) 0)
      (`GameplayStatics.SetGamePaused` true)
      (set `PlayerController.bShowMouseCursor` true (`GameplayStatics.GetPlayerController` 0))
      (bind _returnvalue (`|CreateWidget` "/Game/UI/WB_EndingMenu.WB_EndingMenu_C"))
      (`UserWidget.AddToViewport` _returnvalue 0))))

(fn `UserConstructionScript`)